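; Wave controller for enemy spaceships that, on BeginPlay, sets ship spacing and spawn origin, then runs a hard-coded example scenario.
; The scenario builds waves from squads of ship class and count, exercises add, modify and delete operations, then spawns the first wave.
; Helper functions wrap struct creation and wave calls defined outside these graphs.
; ModifySquadFunction and DeleteSquadFunction are empty, and leftover EventGraph test nodes never run.
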(event EventBeginPlay
  (Variables|Default|SetSpaceshipAdjacence 5e+02)
  (Variables|Default|SetFInitialSpawnPosition (Transformation|GetWorldTransform (Variables|Default|GetDefaultSceneRoot)))
  (CallFunction|GenerateScenarioExample))

(fn ConstructionScript)

(fn CreateWaveFunction
  (params (SpaceshipSquads :type Array%20of%20Spaceship%20Squad%20Structures) (SpawnTime :type Integer))
  (return (Utilities|Struct|MakeSpaceshipWave SpaceshipSquads SpawnTime)))

(fn ModifyWaveFunction
  (params (NumWaveToModify :type Integer) (NewSpaceshipWave :type Spaceship%20Wave%20Structure))
  (Class|WaveController|ModifyWave NumWaveToModify NewSpaceshipWave))

(fn DeleteWaveFunction
  (params (NumWaveToDelete :type Integer))
  (Class|WaveController|DeleteWave NumWaveToDelete))

(fn CreateSquadFunction
  (params (SpaceshipType :type Actor%20Class%20Reference) (NumberOfSpaceship :type Integer))
  (return (Utilities|Struct|MakeSpaceshipSquad SpaceshipType NumberOfSpaceship)))

(fn ModifySquadFunction)

(fn DeleteSquadFunction)

(fn GenerateScenarioExample
  (Utilities|FlowControl|Sequence
    (:then_0
      ;[1 1 1] Create First Wave
      (bind _spaceship_squad (SquadManagement|CreateSquadFunction "/Game/Characters/NPC/Blueprint/BP_WraithEnemyShip.BP_WraithEnemyShip_C" 3))
      (bind _spaceship_squad_2 (SquadManagement|CreateSquadFunction "/Game/Characters/NPC/Blueprint/BP_WraithEnemyShip.BP_WraithEnemyShip_C" 3))
      (bind _spaceship_squad_3 (SquadManagement|CreateSquadFunction "/Game/Characters/NPC/Blueprint/BP_TitanEnemyShip.BP_TitanEnemyShip_C" 1))
      (bind _spaceship_squad_4 (SquadManagement|CreateSquadFunction "/Game/Characters/NPC/Blueprint/BP_WraithEnemyShip.BP_WraithEnemyShip_C" 3))
      (bind _spaceshipwave (WaveManagement|CreateWaveFunction (Utilities|Array|MakeArray _spaceship_squad _spaceship_squad_2 _spaceship_squad_3 _spaceship_squad_4) 3))
      (Class|WaveController|AddWave _spaceshipwave))
    (:then_1
      ;[1 1 1] Modify second squad of the first wave
      (bind _spaceship_squad_5 (SquadManagement|CreateSquadFunction "/Game/Characters/NPC/Blueprint/BP_InterceptorEnemyShip.BP_InterceptorEnemyShip_C" 2))
      (Class|WaveController|ModifySquad 0 1 _spaceship_squad_5))
    (:then_2
      ;[1 1 1] Delete fourth squad of the first wave
      (Class|WaveController|DeleteSquad 0 3))
    (:then_3
      ;[1 1 1] Create second wave
      (bind _spaceship_squad_6 (SquadManagement|CreateSquadFunction "/Game/Characters/NPC/Blueprint/BP_WraithEnemyShip.BP_WraithEnemyShip_C" 3))
      (bind _spaceship_squad_7 (SquadManagement|CreateSquadFunction "/Game/Characters/NPC/Blueprint/BP_InterceptorEnemyShip.BP_InterceptorEnemyShip_C" 3))
      (bind _spaceshipwave_2 (WaveManagement|CreateWaveFunction (Utilities|Array|MakeArray _spaceship_squad_6 _spaceship_squad_7) 50))
      (Class|WaveController|AddWave _spaceshipwave_2))
    (:then_4
      ;[1 1 1] Modify second wave
      (bind _spaceship_squad_8 (SquadManagement|CreateSquadFunction "/Game/Characters/NPC/Blueprint/BP_TitanEnemyShip.BP_TitanEnemyShip_C" 3))
      (bind _spaceship_squad_9 (SquadManagement|CreateSquadFunction "/Game/Characters/NPC/Blueprint/BP_InterceptorEnemyShip.BP_InterceptorEnemyShip_C" 3))
      (bind _spaceshipwave_3 (WaveManagement|CreateWaveFunction (Utilities|Array|MakeArray _spaceship_squad_8 _spaceship_squad_9) 180))
      (Class|WaveController|ModifyWave 1 _spaceshipwave_3))
    (:then_5
      ;[1 1 1] Delete second wave
      (Class|WaveController|DeleteWave 1))
    (:then_6
      ;[1 1 1] Spawn first wave
      (Class|WaveController|GenerateWave))))
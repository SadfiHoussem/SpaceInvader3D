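; BP_Laser is a laser weapon actor that delivers damage to whatever its LaserCollision component overlaps.
; On overlap it ignores itself and its owner, sends its Damage value to actors implementing BPI_IDamageable, then sets a short lifespan on any such hit, damageable or not.
; The FireLaser event only stores a Shooter reference, which the overlap logic does not use.
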(event OnComponentBeginOverlap(LaserCollision)
  (params (OverlappedComponent :type Primitive%20Component%20Object%20Reference) (OtherActor :type Actor%20Object%20Reference) (OtherComp :type Primitive%20Component%20Object%20Reference) (OtherBodyIndex :type Integer) (bFromSweep :type Boolean) (SweepResult :type Hit%20Result%20Structure%20%28by%20ref%29))
  (if (and (!= OtherActor (Components|GetOwner)) (!= OtherActor self))
    (if (Utilities|DoesObjectImplementInterface OtherActor "/Game/Characters/Player/Weapon/BPI_IDamageable.BPI_IDamageable_C")
      (Class|BPIIDamageable|GetDamage(Message) OtherActor (Variables|Weapon|GetDamage)))
    (Actor|SetLifeSpan 0.2)))

(event EventBeginPlay)

(event Collision|EventActorBeginOverlap
  (params (OtherActor :type Actor%20Object%20Reference)))

(event EventTick
  (params (DeltaSeconds :type Float%20%28single-precision%29)))

(event EventFireLaser
  (params (Shooter :type Actor%20Object%20Reference))
  (Variables|Weapon|SetShooter Shooter))

(fn ConstructionScript)
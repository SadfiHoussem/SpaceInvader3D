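; BP_TitanEnemyShip is an enemy ship that shoots lasers at the player and can take hull damage.
; It caches the player pawn on BeginPlay, and each Fire event rotates EnemyAim toward that pawn before spawning a short-lived BP_EnemyLaser from its transform.
; GetDamage forwards incoming damage to TakeHullDamage; the graph contains no trigger for Fire and no active Tick logic.
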(event EventBeginPlay
  (Variables|Default|SetPlayerPawn (Pawn|GetControlledPawn (Game|GetPlayerController 0))))

(event Collision|EventActorBeginOverlap
  (params (OtherActor :type Actor%20Object%20Reference)))

(event EventGetDamage
  (params (Damage :type Float%20%28single-precision%29))
  (Class|AIEnemyShip|TakeHullDamage Damage))

(event EventTick
  (params (DeltaSeconds :type Float%20%28single-precision%29)))

(event EventFire
  (CallFunction|ChangeGunOrientation)
  (bind _returnvalue (Game|SpawnActorfromClass "/Game/Characters/NPC/Weapon/BP_EnemyLaser.BP_EnemyLaser_C" (Transformation|GetWorldTransform (Variables|Default|GetEnemyAim)) "AlwaysSpawn" 0 0))
  (Actor|SetLifeSpan _returnvalue 4.0))

(fn ConstructionScript)

(fn ChangeGunOrientation
  (bind _playerpawn (Variables|Default|GetPlayerPawn))
  (Utilities|IsValid _playerpawn
    (:Is%20Valid
      (Transformation|SetWorldRotation (Variables|Default|GetEnemyAim) (Math|Rotator|FindLookatRotation (.location (Transformation|GetWorldTransform (Variables|Default|GetEnemyAim))) (.location (Transformation|GetWorldTransform (Variables|/Script/Engine.Actor|GetRootComponent _playerpawn)))) false false))))